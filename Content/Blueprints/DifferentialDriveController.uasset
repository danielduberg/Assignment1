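; Controller that drives its pawn along a waypoint list like a differential-drive vehicle, with input to toggle playback or reset to the start.
; Each Tick, it turns yaw toward the current waypoint by at most MaxAngle, then moves the pawn at speed V along its heading, without delta-time scaling.
; An XY tolerance check advances the waypoint index, and playback stops once that index reaches the last entry.
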(event EventBeginPlay
  (bind _waypoints (Variables|Default|Getwaypoints))
  (Variables|Default|SettMax (- (Utilities|Array|Length _waypoints) 1))
  (Input|EnableInput (Game|GetPlayerController 0))
  (Transformation|Teleport (Pawn|GetControlledPawn) (Utilities|Array|Get(acopy) _waypoints) "0, 0, 0"))

(event EventTick
  (params (DeltaSeconds :type Float%20%28single-precision%29))
  (if (Variables|Default|Getplay)
    (bind _reached (CallFunction|WaypointReached))
    (if _reached
      (bind _success (CallFunction|IncrementT))
      (if _success
        (CallFunction|SetVelocity :!label _label)
        (Transformation|SetActorLocation (Pawn|GetControlledPawn) (+ (Utilities|GetCurrentLocation) (Variables|Default|Getvelocity)) false false)
        (else
          (Variables|Default|Setplay false)))
      (else
        (goto _label)))))

(event Input|ActionEvents|InputActionPlayWaypoints
  (params (Key :type Key%20Structure :default "AnyKey"))
  (:Pressed
    (Variables|Default|Setplay (not (Variables|Default|Getplay)))))

(event Input|ActionEvents|InputActionResetPlay
  (params (Key :type Key%20Structure :default "AnyKey"))
  (:Pressed
    (bind _output_get (Variables|Default|Sett 0))
    (Transformation|Teleport (Pawn|GetControlledPawn) (Utilities|Array|Get(acopy) (Variables|Default|Getwaypoints) _output_get) "0, 0, 0")))

(fn ConstructionScript)

(fn WaypointReached
  (bind _location (Utilities|GetCurrentLocation))
  (bind _waypoint (Utilities|GetCurrentWaypoint))
  (return (Math|Vector|Equal(Vector) (Math|Vector|MakeVector (.x _waypoint) (.y _waypoint) 0.0) (Math|Vector|MakeVector (.x _location) (.y _location) 0.0) (LocalVariables|GeterrorTolerance))))

(fn IncrementT
  (if (< (Variables|Default|Gett) (Variables|Default|GettMax))
    (Variables|Default|Sett (+ (Variables|Default|Gett) 1))
    (bind _direction (CallFunction|GetRotation (Utilities|GetCurrentLocation) (Utilities|GetCurrentWaypoint)))
    (Development|PrintString (Utilities|String|ToString(Float) (.yaw _direction))))
  (return (< (Variables|Default|Gett) (Variables|Default|GettMax))))

(fn Rotate
  (bind _returnvalue (Pawn|GetControlledPawn))
  (bind _maxangle (Variables|Default|GetmaxAngle))
  (bind _returnvalue_2 (Transformation|GetActorRotation _returnvalue))
  (bind _direction (CallFunction|GetRotation (Utilities|GetCurrentLocation) (Utilities|GetCurrentWaypoint)))
  (Transformation|SetActorRotation (Pawn|GetControlledPawn) (Math|Rotator|MakeRotator 0.0 0.0 (Math|Float|ClampAngle (.yaw _direction) (- (.yaw _returnvalue_2) _maxangle) (+ _maxangle (.yaw _returnvalue_2))))))

(fn GetRotation
  (params (start :type Vector) (target :type Vector))
  (return (Math|Rotator|MakeRotator 0.0 0.0 (.yaw (Math|Rotator|FindLookatRotation start target)))))

(fn SetVelocity
  (CallFunction|Rotate)
  (bind _xvelocity (CallFunction|GetXVelocity))
  (bind _yvelocity (CallFunction|GetYVelocity))
  (Variables|Default|Setvelocity (Math|Vector|MakeVector _xvelocity _yvelocity 0.0)))

(fn GetXVelocity
  (return (* (Variables|Default|Getv) (Math|Trig|Cos(Degrees) (.yaw (Transformation|GetActorRotation (Pawn|GetControlledPawn)))))))

(fn GetYVelocity
  (return (* (Variables|Default|Getv) (Math|Trig|Sin(Degrees) (.yaw (Transformation|GetActorRotation (Pawn|GetControlledPawn)))))))