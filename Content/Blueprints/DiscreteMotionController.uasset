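; Controller that moves its pawn through a generated waypoint path in discrete teleports.
; On BeginPlay it builds the path with GeneratePath and enables player input for stepping forward or back, toggling playback and resetting to the start.
; Index helpers clamp movement to the path ends, and each step turns the pawn's yaw toward the new waypoint.
; Playback advances on Tick through a short Delay and stops at the last waypoint.
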(event EventBeginPlay
  (bind _returnvalue (Class|AStar|GeneratePath (Variables|Default|GetnumNeighbours)))
  (bind _output_get (Variables|Default|Setwaypoints _returnvalue))
  (Variables|Default|SettMax (- (Utilities|Array|Length _output_get) 1))
  (Input|EnableInput (Game|GetPlayerController 0)))

(event EventTick
  (params (DeltaSeconds :type Float%20%28single-precision%29))
  (if (Variables|Default|Getplay)
    (Utilities|FlowControl|Delay)
    (bind _success (CallFunction|IncrementT))
    (if _success
      (CallFunction|SetLocation)
      (else
        (Variables|Default|Setplay false)))))

(event Input|ActionEvents|InputActionPreviousWaypoint
  (params (Key :type Key%20Structure :default "AnyKey"))
  (:Pressed
    (bind _success (CallFunction|DecrementT))
    (if _success
      (CallFunction|SetLocation))))

(event Input|ActionEvents|InputActionNextWaypoint
  (params (Key :type Key%20Structure :default "AnyKey"))
  (:Pressed
    (bind _success (CallFunction|IncrementT))
    (if _success
      (CallFunction|SetLocation))))

(event Input|ActionEvents|InputActionPlayWaypoints
  (params (Key :type Key%20Structure :default "AnyKey"))
  (:Pressed
    (bind _output_get (Variables|Default|Setplay (not (Variables|Default|Getplay))))
    (if (and _output_get (== (Variables|Default|Gett) (Variables|Default|GettMax)))
      (bind _output_get_2 (Variables|Default|Sett 0))
      (Transformation|Teleport (Pawn|GetControlledPawn) (Utilities|Array|Get(acopy) (Variables|Default|Getwaypoints) _output_get_2) "0, 0, 0"))))

(event Input|ActionEvents|InputActionResetPlay
  (params (Key :type Key%20Structure :default "AnyKey"))
  (:Pressed
    (bind _output_get (Variables|Default|Sett 0))
    (Transformation|Teleport (Pawn|GetControlledPawn) (Utilities|Array|Get(acopy) (Variables|Default|Getwaypoints) _output_get) "0, 0, 0")))

(fn ConstructionScript)

(fn GetRotation
  (params (start :type Vector) (target :type Vector))
  (return (Math|Rotator|MakeRotator 0.0 0.0 (.yaw (Math|Rotator|FindLookatRotation start target)))))

(fn SetLocation
  (bind _returnvalue (Pawn|GetControlledPawn))
  (bind _waypoints (Variables|Default|Getwaypoints))
  (bind _t (Variables|Default|Gett))
  (bind _item (Utilities|Array|Get(acopy) _waypoints _t))
  (bind _direction (CallFunction|GetRotation (Transformation|GetActorLocation _returnvalue) _item))
  (Transformation|Teleport _returnvalue _item _direction))

(fn DecrementT
  (if (> (Variables|Default|Gett) 0)
    (Variables|Default|Sett (- (Variables|Default|Gett) 1))
    (return true)
    (else
      (return false))))

(fn IncrementT
  (if (< (Variables|Default|Gett) (Variables|Default|GettMax))
    (Variables|Default|Sett (+ (Variables|Default|Gett) 1))
    (return true)
    (else
      (return false))))