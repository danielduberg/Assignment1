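; Controller that drives a car pawn along a waypoint list using a kinematic steering model, with input to play/pause and reset.
; Each tick it advances the waypoint within an XY tolerance, stopping when the index reaches the last one.
; Steering clamps look-at yaw to a maximum angle, turns by tan(angle)·V/L, then derives velocity from the heading.
; Movement sets location directly per frame, without sweep or delta-time scaling.
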(event EventBeginPlay
  (Variables|Default|SettMax (- (Utilities|Array|Length (Variables|Default|Getwaypoints)) 1))
  (Input|EnableInput (Game|GetPlayerController 0)))

(event EventTick
  (params (DeltaSeconds :type Float%20%28single-precision%29))
  (bind _returnvalue (Pawn|GetControlledPawn))
  (if (Variables|Default|Getplay)
    (bind _reached (CallFunction|WaypointReached))
    (if _reached
      (bind _success (CallFunction|IncrementT))
      (if _success
        (CallFunction|SetVelocity :!label _label)
        (Transformation|SetActorLocation _returnvalue (+ (Utilities|GetCurrentLocation) (Variables|Default|Getvelocity)) false false)
        (Development|PrintString (Utilities|String|ToString(Vector) (Transformation|GetActorLocation _returnvalue)) true true "(R=0.000000,G=0.660000,B=1.000000,A=1.000000)" 2e+04)
        (else
          (Variables|Default|Setplay false)))
      (else
        (goto _label)))))

(event Input|ActionEvents|InputActionPlayWaypoints
  (params (Key :type Key%20Structure :default "AnyKey"))
  (:Pressed
    (bind _output_get (Variables|Default|Setplay (not (Variables|Default|Getplay))))
    (if (and _output_get (== (Variables|Default|Gett) (Variables|Default|GettMax)))
      (bind _output_get_2 (Variables|Default|Sett 0))
      (Transformation|Teleport (Pawn|GetControlledPawn) (Utilities|Array|Get(acopy) (Variables|Default|Getwaypoints) _output_get_2) "0, 0, 0"))))

(event Input|ActionEvents|InputActionResetPlay
  (params (Key :type Key%20Structure :default "AnyKey"))
  (:Pressed
    (bind _output_get (Variables|Default|Sett 0))
    (Transformation|Teleport (Pawn|GetControlledPawn) (Utilities|Array|Get(acopy) (Variables|Default|Getwaypoints) _output_get) "0, 0, 0")))

(fn ConstructionScript)

(fn WaypointReached
  (bind _location (Utilities|GetCurrentLocation))
  (bind _waypoint (Utilities|GetCurrentWaypoint))
  (return (Math|Vector|Equal(Vector) (Math|Vector|MakeVector (.x _waypoint) (.y _waypoint) 0.0) (Math|Vector|MakeVector (.x _location) (.y _location) 0.0) (LocalVariables|GeterrorTolerance))))

(fn IncrementT
  (if (< (Variables|Default|Gett) (Variables|Default|GettMax))
    (Variables|Default|Sett (+ (Variables|Default|Gett) 1)))
  (return (< (Variables|Default|Gett) (Variables|Default|GettMax))))

(fn Rotate
  (bind _returnvalue (Pawn|GetControlledPawn))
  (bind _maxangle (Variables|Default|GetmaxAngle))
  (bind _returnvalue_2 (Transformation|GetActorRotation _returnvalue))
  (bind _direction (CallFunction|GetRotation (Utilities|GetCurrentLocation) (Utilities|GetCurrentWaypoint)))
  (Transformation|SetActorRotation (Pawn|GetControlledPawn) (Math|Rotator|MakeRotator 0.0 0.0 (+ (* (Math|Trig|Tan(Degrees) (- (Math|Float|ClampAngle (.yaw _direction) (- (.yaw _returnvalue_2) _maxangle) (+ _maxangle (.yaw _returnvalue_2))) (.yaw _returnvalue_2))) (/ (Variables|Default|Getv) (Variables|Default|GetL))) (.yaw _returnvalue_2))))
  (return (+ (* (Math|Trig|Tan(Degrees) (- (Math|Float|ClampAngle (.yaw _direction) (- (.yaw _returnvalue_2) _maxangle) (+ _maxangle (.yaw _returnvalue_2))) (.yaw _returnvalue_2))) (/ (Variables|Default|Getv) (Variables|Default|GetL))) (.yaw _returnvalue_2))))

(fn GetRotation
  (params (start :type Vector) (target :type Vector))
  (return (Math|Rotator|MakeRotator 0.0 0.0 (.yaw (Math|Rotator|FindLookatRotation start target)))))

(fn SetVelocity
  (bind _angle (CallFunction|Rotate))
  (bind _xvelocity (CallFunction|GetXVelocity _angle))
  (bind _yvelocity (CallFunction|GetYVelocity _angle))
  (Variables|Default|Setvelocity (Math|Vector|MakeVector _xvelocity _yvelocity 0.0)))

(fn GetXVelocity
  (params (angle :type Float%20%28single-precision%29))
  (return (* (Math|Trig|Cos(Degrees) angle) (Variables|Default|Getv))))

(fn GetYVelocity
  (params (angle :type Float%20%28single-precision%29))
  (return (* (Math|Trig|Sin(Degrees) angle) (Variables|Default|Getv))))