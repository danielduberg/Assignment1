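; Controller that drives its pawn through generated waypoints as a dynamic point mass with limited acceleration and speed.
; Each tick SetAcceleration steers toward the current waypoint, braking when aligned and within stopping distance, then velocity is integrated to move and yaw the pawn.
; WaypointReached uses an XY tolerance, usually zeroing velocity before IncrementT advances the index.
; Input toggles playback or resets to the first waypoint, while elapsed time prints on screen.
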(event EventBeginPlay
  (bind _location (Utilities|GetCurrentLocation))
  (bind _returnvalue (Class|AStar|GeneratePath2))
  (bind _output_get (Variables|Default|Setwaypoints _returnvalue))
  (Variables|Default|SettMax (- (Utilities|Array|Length _output_get) 1))
  (Input|EnableInput (Game|GetPlayerController 0))
  (Transformation|SetActorRotation (Pawn|GetControlledPawn) (Math|Rotator|FindLookatRotation (Math|Vector|MakeVector (.x _location) (.y _location) 0.0) (Math|Vector|MakeVector (.x (Utilities|Array|Get(acopy) _output_get 1)) (.y (Utilities|Array|Get(acopy) _output_get 1)) 0.0))))

(event EventTick
  (params (DeltaSeconds :type Float%20%28single-precision%29))
  (bind _vmax (Variables|Default|GetvMax))
  (if (Variables|Default|Getplay)
    (bind _output_get (Variables|Default|SettimeTaken (+ DeltaSeconds (Variables|Default|GettimeTaken))))
    (Development|PrintString (Utilities|String|ToString(Float) _output_get) true true "(R=0.000000,G=0.660000,B=1.000000,A=1.000000)" 2e+01)
    (bind _reached (CallFunction|WaypointReached))
    (if _reached
      (bind _success (CallFunction|IncrementT))
      (if (not _success)
        (Variables|Default|Setplay false))
      (else
        (bind _acceleration (CallFunction|SetAcceleration))
        (bind _output_get_2 (Variables|Default|Setacceleration _acceleration))
        (bind _output_get_3 (Variables|Default|Setvelocity (Math|Vector|ClampVectorSize (+ (* _output_get_2 (Utilities|Time|GetWorldDeltaSeconds)) (Variables|Default|Getvelocity)) (* _vmax -1.0) _vmax)))
        (CallFunction|SetRotation)
        (Transformation|SetActorLocationAndRotation (Pawn|GetControlledPawn) (+ (* _output_get_3 (Utilities|Time|GetWorldDeltaSeconds)) (Utilities|GetCurrentLocation)) (Transformation|GetActorRotation (Pawn|GetControlledPawn)) true true)))))

(event Input|ActionEvents|InputActionPlayWaypoints
  (params (Key :type Key%20Structure :default "AnyKey"))
  (bind _location (Utilities|GetCurrentLocation))
  (bind _waypoints (Variables|Default|Getwaypoints))
  (bind _item (Utilities|Array|Get(acopy) _waypoints 1))
  (:Pressed
    (bind _output_get (Variables|Default|Setplay (not (Variables|Default|Getplay))))
    (if (and _output_get (== (Variables|Default|Gett) (Variables|Default|GettMax)))
      (Variables|Default|Setvelocity "0, 0, 0")
      (bind _output_get_2 (Variables|Default|Sett 0))
      (Transformation|Teleport (Pawn|GetControlledPawn) (Utilities|Array|Get(acopy) (Variables|Default|Getwaypoints) _output_get_2) (Math|Rotator|FindLookatRotation (Math|Vector|MakeVector (.x _location) (.y _location) 0.0) (Math|Vector|MakeVector (.x _item) (.y _item) 0.0))))))

(event Input|ActionEvents|InputActionResetPlay
  (params (Key :type Key%20Structure :default "AnyKey"))
  (bind _location (Utilities|GetCurrentLocation))
  (bind _waypoints (Variables|Default|Getwaypoints))
  (bind _item (Utilities|Array|Get(acopy) _waypoints 1))
  (:Pressed
    (Variables|Default|Setvelocity "0, 0, 0")
    (bind _output_get (Variables|Default|Sett 0))
    (Transformation|Teleport (Pawn|GetControlledPawn) (Utilities|Array|Get(acopy) (Variables|Default|Getwaypoints) _output_get) (Math|Rotator|FindLookatRotation (Math|Vector|MakeVector (.x _location) (.y _location) 0.0) (Math|Vector|MakeVector (.x _item) (.y _item) 0.0)))))

(fn ConstructionScript)

(fn IncrementT
  (if (< (Variables|Default|Gett) (Variables|Default|GettMax))
    (Variables|Default|Sett (+ (Variables|Default|Gett) 1))
    (return true)
    (else
      (return false))))

(fn GetRotation
  (params (start :type Vector) (target :type Vector))
  (return (Math|Rotator|MakeRotator 0.0 0.0 (.yaw (Math|Rotator|FindLookatRotation start target)))))

(fn WaypointReached
  (bind _location (Utilities|GetCurrentLocation))
  (bind _waypoint (Utilities|GetCurrentWaypoint))
  (bind _errortolerance (LocalVariables|GeterrorTolerance))
  (bind _returnvalue (Math|Vector|Equal(Vector) (Math|Vector|MakeVector (.x _waypoint) (.y _waypoint) 0.0) (Math|Vector|MakeVector (.x _location) (.y _location) 0.0) _errortolerance))
  (Development|PrintString (Utilities|String|ToString(Vector) (Utilities|GetCurrentLocation)) false)
  (Development|PrintString (Utilities|String|ToString(Vector) (Utilities|GetCurrentWaypoint)) false true "(R=1.000000,G=0.000000,B=0.137657,A=1.000000)")
  (if _returnvalue
    (bind _acceleration (CallFunction|SetAcceleration))
    (if (> (Math|Float|Absolute(Float) (.x (* _acceleration (Utilities|Time|GetWorldDeltaSeconds)))) (Math|Float|Absolute(Float) (.x (* (Variables|Default|Getvelocity) (Utilities|Time|GetWorldDeltaSeconds)))))
      (if (> (Math|Float|Absolute(Float) (.y (* _acceleration (Utilities|Time|GetWorldDeltaSeconds)))) (Math|Float|Absolute(Float) (.y (* (Variables|Default|Getvelocity) (Utilities|Time|GetWorldDeltaSeconds)))))
        (Variables|Default|Setvelocity "0, 0, 0")
        (return true)
        (else
          _)))
    (return false)
    (else
      (return _returnvalue))))

(fn SetAcceleration
  (bind _location (Utilities|GetCurrentLocation))
  (bind _waypoint (Utilities|GetCurrentWaypoint))
  (bind _waypoint_2 (Utilities|GetCurrentWaypoint))
  (bind _location_2 (Utilities|GetCurrentLocation))
  (bind _velocity (Variables|Default|Getvelocity))
  (bind _velocity_2 (Variables|Default|Getvelocity))
  (bind _returnvalue (Math|Vector|VectorLength _velocity_2))
  (bind _returnvalue_2 (- (Math|Vector|MakeVector (.x _waypoint_2) (.y _waypoint_2) 0.0) (Math|Vector|MakeVector (.x _location_2) (.y _location_2) 0.0)))
  (bind _direction (CallFunction|GetRotation (Utilities|GetCurrentLocation) (Utilities|GetCurrentWaypoint)))
  (if (>= (/ (* _returnvalue _returnvalue) (* (Variables|Default|GetaMax) 2.0)) (- (Math|Vector|VectorLength (- (Math|Vector|MakeVector (.x _waypoint) (.y _waypoint) 0.0) (Math|Vector|MakeVector (.x _location) (.y _location) 0.0))) (LocalVariables|GetsafetyBuffer)))
    (if (Math|Vector|Equal(Vector) (Math|Conversions|ToVector(Vector2D) (Math|Vector2D|Normalize2D (Math|Vector2D|MakeVector2D (.x _velocity) (.y _velocity)))) (Math|Conversions|ToVector(Vector2D) (Math|Vector2D|Normalize2D (Math|Vector2D|MakeVector2D (.x _returnvalue_2) (.y _returnvalue_2)))) 0.1)
      (bind _output_get (Variables|Default|Setacceleration (* (* (/ (Math|Vector|MakeVector (Math|Trig|Cos(Degrees) (.yaw _direction)) (Math|Trig|Sin(Degrees) (.yaw _direction)) 0.0) (Variables|Default|Getmass)) (Variables|Default|GetaMax)) -1.0)))
      (return _output_get)
      (else
        _)))
  (bind _output_get_2 (Variables|Default|Setacceleration (* (/ (Math|Vector|MakeVector (Math|Trig|Cos(Degrees) (.yaw _direction)) (Math|Trig|Sin(Degrees) (.yaw _direction)) 0.0) (Variables|Default|Getmass)) (Variables|Default|GetaMax))))
  (return _output_get_2))

(fn SetRotation
  (bind _velocity (Variables|Default|Getvelocity))
  (bind _returnvalue (Math|Vector|Normalize _velocity))
  (Transformation|SetActorRotation (Pawn|GetControlledPawn) (Math|Rotator|MakeRotator 0.0 0.0 (Class|KismetMathLibrary|DegAtan2 (.y _returnvalue) (.x _returnvalue)))))