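; Controller that drives its pawn along a generated waypoint path using a kinematic car model, with input to play, pause and reset.
; Each tick prints elapsed play time, advances the waypoint when within tolerance, and stops after the last.
; Rotate derives yaw from the tangent of a rate-clamped look-at angle times VMax over L, applying it directly as absolute yaw.
; SetVelocity converts that yaw into constant-speed XY velocity, moving the pawn without sweeping.
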(event EventBeginPlay
  (bind _location (Utilities|GetCurrentLocation))
  (bind _returnvalue (Class|AStar|GeneratePath2 (Variables|Default|Getbuffer)))
  (bind _output_get (Variables|Default|Setwaypoints _returnvalue))
  (Variables|Default|SettMax (- (Utilities|Array|Length _output_get) 1))
  (Input|EnableInput (Game|GetPlayerController 0))
  (Transformation|SetActorRotation (Pawn|GetControlledPawn) (Math|Rotator|FindLookatRotation (Math|Vector|MakeVector (.x _location) (.y _location) 0.0) (Math|Vector|MakeVector (.x (Utilities|Array|Get(acopy) _output_get 1)) (.y (Utilities|Array|Get(acopy) _output_get 1)) 0.0))))

(event EventTick
  (params (DeltaSeconds :type Float%20%28single-precision%29))
  (if (Variables|Default|Getplay)
    (bind _output_get (Variables|Default|SettimeTaken (+ DeltaSeconds (Variables|Default|GettimeTaken))))
    (Development|PrintString (Utilities|String|ToString(Float) _output_get) true true "(R=0.000000,G=0.660000,B=1.000000,A=1.000000)" 2e+01)
    (bind _reached (CallFunction|WaypointReached))
    (if _reached
      (bind _success (CallFunction|IncrementT))
      (if _success
        (bind _velocity (CallFunction|SetVelocity :!label _label))
        (bind _output_get_2 (Variables|Default|Setvelocity _velocity))
        (Transformation|SetActorLocation (Pawn|GetControlledPawn) (+ (* _output_get_2 (Utilities|Time|GetWorldDeltaSeconds)) (Utilities|GetCurrentLocation)) false false)
        (else
          (Variables|Default|Setplay false)))
      (else
        (goto _label)))))

(event Input|ActionEvents|InputActionPlayWaypoints
  (params (Key :type Key%20Structure :default "AnyKey"))
  (bind _location (Utilities|GetCurrentLocation))
  (bind _waypoints (Variables|Default|Getwaypoints))
  (bind _item (Utilities|Array|Get(acopy) _waypoints 1))
  (:Pressed
    (bind _output_get (Variables|Default|Setplay (not (Variables|Default|Getplay))))
    (if (and _output_get (== (Variables|Default|Gett) (Variables|Default|GettMax)))
      (Variables|Default|Setvelocity "0, 0, 0")
      (bind _output_get_2 (Variables|Default|Sett 0))
      (Transformation|Teleport (Pawn|GetControlledPawn) (Utilities|Array|Get(acopy) (Variables|Default|Getwaypoints) _output_get_2) (Math|Rotator|FindLookatRotation (Math|Vector|MakeVector (.x _location) (.y _location) 0.0) (Math|Vector|MakeVector (.x _item) (.y _item) 0.0))))))

(event Input|ActionEvents|InputActionResetPlay
  (params (Key :type Key%20Structure :default "AnyKey"))
  (bind _location (Utilities|GetCurrentLocation))
  (bind _waypoints (Variables|Default|Getwaypoints))
  (bind _item (Utilities|Array|Get(acopy) _waypoints 1))
  (:Pressed
    (Variables|Default|Setvelocity "0, 0, 0")
    (bind _output_get (Variables|Default|Sett 0))
    (Transformation|Teleport (Pawn|GetControlledPawn) (Utilities|Array|Get(acopy) (Variables|Default|Getwaypoints) _output_get) (Math|Rotator|FindLookatRotation (Math|Vector|MakeVector (.x _location) (.y _location) 0.0) (Math|Vector|MakeVector (.x _item) (.y _item) 0.0)))))

(fn ConstructionScript)

(fn WaypointReached
  (bind _location (Utilities|GetCurrentLocation))
  (bind _waypoint (Utilities|GetCurrentWaypoint))
  (return (Math|Vector|Equal(Vector) (Math|Vector|MakeVector (.x _waypoint) (.y _waypoint) 0.0) (Math|Vector|MakeVector (.x _location) (.y _location) 0.0) (LocalVariables|GeterrorTolerance))))

(fn IncrementT
  (if (< (Variables|Default|Gett) (Variables|Default|GettMax))
    (Variables|Default|Sett (+ (Variables|Default|Gett) 1))
    (return true)
    (else
      (return false))))

(fn Rotate
  (bind _returnvalue (Utilities|Time|GetWorldDeltaSeconds))
  (bind _returnvalue_2 (Pawn|GetControlledPawn))
  (bind _maxangle (Variables|Default|GetmaxAngle))
  (bind _returnvalue_3 (Transformation|GetActorRotation _returnvalue_2))
  (bind _returnvalue_4 (* _maxangle _returnvalue))
  (bind _direction (CallFunction|GetRotation (Utilities|GetCurrentLocation) (Utilities|GetCurrentWaypoint)))
  (Transformation|SetActorRotation (Pawn|GetControlledPawn) (Math|Rotator|MakeRotator 0.0 0.0 (* (Math|Trig|Tan(Degrees) (Math|Float|ClampAngle (.yaw _direction) (- (.yaw _returnvalue_3) _returnvalue_4) (+ _returnvalue_4 (.yaw _returnvalue_3)))) (/ (Variables|Default|GetvMax) (Variables|Default|GetL)))))
  (return (* (Math|Trig|Tan(Degrees) (Math|Float|ClampAngle (.yaw _direction) (- (.yaw _returnvalue_3) _returnvalue_4) (+ _returnvalue_4 (.yaw _returnvalue_3)))) (/ (Variables|Default|GetvMax) (Variables|Default|GetL)))))

(fn GetRotation
  (params (start :type Vector) (target :type Vector))
  (return (Math|Rotator|MakeRotator 0.0 0.0 (.yaw (Math|Rotator|FindLookatRotation start target)))))

(fn SetVelocity
  (bind _angle (CallFunction|Rotate))
  (bind _xvelocity (CallFunction|GetXVelocity _angle))
  (bind _yvelocity (CallFunction|GetYVelocity _angle))
  (return (Math|Vector|MakeVector _xvelocity _yvelocity 0.0)))

(fn GetXVelocity
  (params (angle :type Float%20%28single-precision%29))
  (return (* (Math|Trig|Cos(Degrees) angle) (Variables|Default|GetvMax))))

(fn GetYVelocity
  (params (angle :type Float%20%28single-precision%29))
  (return (* (Math|Trig|Sin(Degrees) angle) (Variables|Default|GetvMax))))