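; Controller that drives its pawn along a generated list of waypoints as a kinematic point.
; While playing, Tick faces the pawn at the current waypoint and teleports it by a fixed-speed step each frame, without delta-time scaling.
; Each axis of the step is clamped to the remaining distance to avoid overshoot, and the index advances within an error tolerance.
; Input actions toggle playback and reset to the first waypoint.
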(event EventBeginPlay
  (bind _currentlocation (Utilities|GetCurrentLocation))
  (bind _returnvalue (Class|AStar|GeneratePath2))
  (bind _output_get (Variables|Default|Setwaypoints _returnvalue))
  (Variables|Default|SettMax (- (Utilities|Array|Length _output_get) 1))
  (Input|EnableInput (Game|GetPlayerController 0))
  (Transformation|SetActorRotation (Pawn|GetControlledPawn) (Math|Rotator|FindLookatRotation (Math|Vector|MakeVector (.x _currentlocation) (.y _currentlocation) 0.0) (Math|Vector|MakeVector (.x (Utilities|Array|Get(acopy) _output_get 1)) (.y (Utilities|Array|Get(acopy) _output_get 1)) 0.0))))

(event EventTick
  (params (DeltaSeconds :type Float%20%28single-precision%29))
  (bind _returnvalue (Pawn|GetControlledPawn))
  (if (Variables|Default|Getplay)
    (bind _reached (CallFunction|WaypointReached))
    (if _reached
      (bind _success (CallFunction|IncrementT))
      (if _success
        (CallFunction|SetVelocity :!label _label)
        (Transformation|Teleport _returnvalue (+ (Utilities|GetCurrentLocation) (Variables|Default|Getvelocity)) (Transformation|GetActorRotation _returnvalue))
        (else
          (Variables|Default|Setplay false)))
      (else
        (goto _label)))))

(event Input|ActionEvents|InputActionPlayWaypoints
  (params (Key :type Key%20Structure :default "AnyKey"))
  (bind _currentlocation (Utilities|GetCurrentLocation))
  (bind _waypoints (Variables|Default|Getwaypoints))
  (bind _item (Utilities|Array|Get(acopy) _waypoints 1))
  (:Pressed
    (bind _output_get (Variables|Default|Setplay (not (Variables|Default|Getplay))))
    (if (and _output_get (== (Variables|Default|Gett) (Variables|Default|GettMax)))
      (bind _output_get_2 (Variables|Default|Sett 0))
      (Transformation|Teleport (Pawn|GetControlledPawn) (Utilities|Array|Get(acopy) (Variables|Default|Getwaypoints) _output_get_2) (Math|Rotator|FindLookatRotation (Math|Vector|MakeVector (.x _currentlocation) (.y _currentlocation) 0.0) (Math|Vector|MakeVector (.x _item) (.y _item) 0.0))))))

(event Input|ActionEvents|InputActionResetPlay
  (params (Key :type Key%20Structure :default "AnyKey"))
  (bind _currentlocation (Utilities|GetCurrentLocation))
  (bind _waypoints (Variables|Default|Getwaypoints))
  (bind _item (Utilities|Array|Get(acopy) _waypoints 1))
  (:Pressed
    (bind _output_get (Variables|Default|Sett 0))
    (Transformation|Teleport (Pawn|GetControlledPawn) (Utilities|Array|Get(acopy) (Variables|Default|Getwaypoints) _output_get) (Math|Rotator|FindLookatRotation (Math|Vector|MakeVector (.x _currentlocation) (.y _currentlocation) 0.0) (Math|Vector|MakeVector (.x _item) (.y _item) 0.0)))))

(fn ConstructionScript)

(fn IncrementT
  (if (< (Variables|Default|Gett) (Variables|Default|GettMax))
    (Variables|Default|Sett (+ (Variables|Default|Gett) 1))
    (return true)
    (else
      (return false))))

(fn GetRotation
  (params (start :type Vector) (target :type Vector))
  (return (Math|Rotator|MakeRotator 0.0 0.0 (.yaw (Math|Rotator|FindLookatRotation start target)))))

(fn SetVelocity
  (bind _waypoint (Utilities|GetCurrentWaypoint))
  (bind _currentlocation (Utilities|GetCurrentLocation))
  (bind _returnvalue (- _waypoint _currentlocation))
  (bind _returnvalue_2 (Math|Float|Absolute(Float) (.y _returnvalue)))
  (bind _returnvalue_3 (Math|Float|Absolute(Float) (.x _returnvalue)))
  (bind _direction (CallFunction|GetRotation _currentlocation _waypoint))
  (Transformation|SetActorRotation (Pawn|GetControlledPawn) (Math|Rotator|MakeRotator 0.0 0.0 (.yaw _direction)))
  (Variables|Default|Setvelocity (Math|Vector|MakeVector (Math|Float|Clamp(Float) (.x (* (Math|Vector|MakeVector (Math|Trig|Cos(Degrees) (.yaw _direction)) (Math|Trig|Sin(Degrees) (.yaw _direction)) 0.0) (Variables|Default|Getv))) (* _returnvalue_3 -1.0) _returnvalue_3) (Math|Float|Clamp(Float) (.y (* (Math|Vector|MakeVector (Math|Trig|Cos(Degrees) (.yaw _direction)) (Math|Trig|Sin(Degrees) (.yaw _direction)) 0.0) (Variables|Default|Getv))) (* _returnvalue_2 -1.0) _returnvalue_2) 0.0)))

(fn WaypointReached
  (bind _waypoint (Utilities|GetCurrentWaypoint))
  (bind _currentlocation (Utilities|GetCurrentLocation))
  (return (Math|Vector|Equal(Vector) (Math|Vector|MakeVector (.x _waypoint) (.y _waypoint) 0.0) (Math|Vector|MakeVector (.x _currentlocation) (.y _currentlocation) 0.0) (LocalVariables|GeterrorTolerance))))

(fn AdjustVelocity
  (CallFunction|AdjustXVelocity)
  (CallFunction|AdjustYVelocity)
  (return))

(fn AdjustXVelocity
  (bind _currentlocation (Utilities|GetCurrentLocation))
  (bind _waypoint (Utilities|GetCurrentWaypoint))
  (bind _returnvalue (- (.x _waypoint) (.x _currentlocation)))
  (bind _returnvalue_2 (Math|Float|Absolute(Float) _returnvalue))
  (Variables|Default|Setvelocity (Math|Vector|MakeVector (Math|Float|Clamp(Float) (.x (Variables|Default|Getvelocity)) (* _returnvalue_2 -1.0) _returnvalue_2) (.y (Variables|Default|Getvelocity)) 0.0))
  (return))

(fn AdjustYVelocity
  (bind _currentlocation (Utilities|GetCurrentLocation))
  (bind _waypoint (Utilities|GetCurrentWaypoint))
  (bind _returnvalue (- (.y _waypoint) (.y _currentlocation)))
  (bind _returnvalue_2 (Math|Float|Absolute(Float) _returnvalue))
  (Variables|Default|Setvelocity (Math|Vector|MakeVector (.x (Variables|Default|Getvelocity)) (Math|Float|Clamp(Float) (.y (Variables|Default|Getvelocity)) (* _returnvalue_2 -1.0) _returnvalue_2) 0.0))
  (return))